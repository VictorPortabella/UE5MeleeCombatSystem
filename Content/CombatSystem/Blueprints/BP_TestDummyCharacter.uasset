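; Test dummy character for the combat system that takes point damage and reacts to hits.
; On BeginPlay it spawns and equips its StartEquipment actors, then prints one current stat from its StatsComponent.
; Point damage goes to StatsComponent, with an impact sound and emitter at the hit location.
; When a hit reaction is allowed, it plays a front-react montage and changes state through StateManagerComponent.
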(event `self.ReceiveBeginPlay`
  (`parent.ReceiveBeginPlay`)
  (for _array_element (`self.StartEquipment`)
    (bind _returnvalue (`|SpawnActorFromClass` _array_element (`self.GetTransform`) "Undefined" "MultiplyWithRoot" self self))
    (`/Game/CombatSystem/Blueprints/Actors/BP_BaseEquippable.OnEquipped` _returnvalue))
  (`KismetSystemLibrary.PrintString` (`KismetStringLibrary.Conv_DoubleToString` (`/Game/CombatSystem/Blueprints/Components/BP_StatsComponent.GetCurrentStatValue` (`self.StatsComponent`) "NewEnumerator3"))))

(event `self.ReceivePointDamage`
  (params (Damage :type "Float (single-precision)") (DamageType :type "DamageType Object Reference") (HitLocation :type "Vector Structure") (HitNormal :type "Vector Structure") (HitComponent :type "PrimitiveComponent Object Reference") (BoneName :type Name) (ShotFromDirection :type "Vector Structure") (InstigatedBy :type "Controller Object Reference") (DamageCauser :type "Actor Object Reference") (HitInfo :type "HitResult Structure (by ref)"))
  ;[1 0.1349 0.1249] Receive Damage
  (`/Game/CombatSystem/Blueprints/Components/BP_StatsComponent.TakeDamage` (`self.StatsComponent`) Damage)
  (`GameplayStatics.PlaySoundAtLocation` "/Game/CombatSystem/CourseFiles/SoundFX/Gruntling/A_Guardian_Impact_Cue.A_Guardian_Impact_Cue" HitLocation (struct) 1.0 1.0 0.0 null null null null)
  (`GameplayStatics.SpawnEmitterAtLocation` null HitLocation (struct) (0.5 0.5 0.5))
  (if (`self.CanReceivedHitReaction`)
    (`self.PlayAnimMontage` "/Game/Characters/Mannequin_UE4/UE4_MannyAnims/UE4Standing_React_Large_Front_Montage.UE4Standing_React_Large_Front_Montage")
    (`/Game/CombatSystem/Blueprints/Components/BP_StateManagerComponent.SetState` (`self.StateManagerComponent`) "NewEnumerator5")))

(fn `UserConstructionScript`
  (`parent.UserConstructionScript`))