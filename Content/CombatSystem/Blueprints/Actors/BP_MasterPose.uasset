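; Base-style equippable armor actor that follows the owning character's animation through leader pose and modifies the owner's stats.
; AttachActor snaps the item's skeletal mesh, if it has an asset, to a socket on the owner Character's mesh and sets that mesh as leader pose component.
; OnEquipped and OnUnequipped extend the parent logic by adding or subtracting ArmorValue on a stat in the owner's BP_StatsComponent.
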(fn `AttachActor`
  (params (SocketName :type Name))
  (bind _mesh (`Character.Mesh` (cast `Character` (`self.GetOwner`) :!pure true)))
  (`/Engine/EditorBlueprintResources/StandardMacros.IsValid` (`SkeletalMeshComponent.SkeletalMeshAsset` (`self.ItemSkeletalMesh`))
    (:`Is Valid`
      (`SceneComponent.K2_AttachToComponent` (`self.ItemSkeletalMesh`) _mesh (`local.SocketName`) "SnapToTarget" "SnapToTarget" "SnapToTarget" true)
      (`SkinnedMeshComponent.SetLeaderPoseComponent` (`self.ItemSkeletalMesh`) _mesh false false)
      (return))))

(fn `OnEquipped`
  (`parent.OnEquipped`)
  (`/Game/CombatSystem/Blueprints/Components/BP_StatsComponent.ModifyCurrentStatValue` (`self.GetComponentByClass` (`self.GetOwner`) "/Game/CombatSystem/Blueprints/Components/BP_StatsComponent.BP_StatsComponent_C") "NewEnumerator3" (`self.ArmorValue`) false))

(fn `OnUnequipped`
  (`parent.OnUnequipped`)
  (`/Game/CombatSystem/Blueprints/Components/BP_StatsComponent.ModifyCurrentStatValue` (`self.GetComponentByClass` (`self.GetOwner`) "/Game/CombatSystem/Blueprints/Components/BP_StatsComponent.BP_StatsComponent_C") "NewEnumerator3" (* (`self.ArmorValue`) -1.0) false))

(fn `UserConstructionScript`
  (`parent.UserConstructionScript`))