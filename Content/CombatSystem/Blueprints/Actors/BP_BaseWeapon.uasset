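; BP_BaseWeapon is the base equippable weapon of the combat system, holding damage, combat type and montages for attacks, dodges and entering or exiting combat.
; On equip it attaches to a hand or stowed socket by combat state, registers as main weapon and sends its combat type to the AnimInstance.
; Its collision component traces the item mesh, ignoring the owner, and hits apply point damage to actors that accept it.
; It can also switch the mesh to physics simulation.
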(event `self.BP_CollisionComponent.OnHit`
  (params (HitResult :type "HitResult Structure"))
  (bind (_bblockinghit _binitialoverlap _time _distance _location _impactpoint _normal _impactnormal _physmat _hitactor) (`GameplayStatics.BreakHitResult` HitResult))
  (bind _canreceivedamage (message `/Game/CombatSystem/Blueprints/Interfaces/Combat_BPI.CanReceiveDamage` _hitactor))
  (if _canreceivedamage
    (`GameplayStatics.ApplyPointDamage` _hitactor (`self.Damage`) (`self.GetActorForwardVector` (`self.GetOwner`)) HitResult (`self.GetInstigatorController`) self)))

(event `SimulateWeaponPhysics`
  (bind _returnvalue (`self.GetItemMesh`))
  (`PrimitiveComponent.SetCollisionProfileName` _returnvalue "PhysicsActor" true)
  (`PrimitiveComponent.SetSimulatePhysics` _returnvalue true))

(fn `GetActionMontages`
  (params (CharacterAction :type "/Game/CombatSystem/Blueprints/Enums/E_CharacterAction Enum" :default "NewEnumerator0"))
  (returns (Montages :type "Array of AnimMontage Object Reference"))
  (return (select `/Game/CombatSystem/Blueprints/Enums/E_CharacterAction` CharacterAction :`NewEnumerator1` (`self.LightAttackMontages`) :`NewEnumerator2` (`self.HeavyAttackMontages`) :`NewEnumerator3` (`self.ChargedAttackMontages`) :`NewEnumerator4` (`self.FallingAttackMontages`) :`NewEnumerator9` (`self.SprintAttackMontages`) :`NewEnumerator5` (`self.DodgeMontages`) :`NewEnumerator6` (`|MakeArray` (`self.EnterCombatMontage`)) :`NewEnumerator7` (`|MakeArray` (`self.ExitCombatMontage`)))))

(fn `OnEquipped`
  (bind _bp_collisioncomponent (`self.BP_CollisionComponent`))
  (`parent.OnEquipped`)
  (set `self.CombatComponent` (`self.GetComponentByClass` (`self.GetOwner`) "/Game/CombatSystem/Blueprints/Components/BP_CombatComponent.BP_CombatComponent_C"))
  (`self.AttachActor` (select `bool` (`/Game/CombatSystem/Blueprints/Components/BP_CombatComponent.GetIsCombatEnabled` (`self.CombatComponent`)) :`false` (`self.AttachSocketName`) :`true` (`self.HandSocketName`)))
  (`/Game/CombatSystem/Blueprints/Components/BP_CombatComponent.SetMainWeapon` (`self.CombatComponent`) self)
  (message `/Game/CombatSystem/Blueprints/Interfaces/AnimInstance_BPI.UpdateCombatType` (`SkeletalMeshComponent.GetAnimInstance` (`Character.Mesh` (cast `Character` (`self.GetOwner`) :!pure true))) (`self.CombatType`))
  (`/Game/CombatSystem/Blueprints/Components/BP_CollisionComponent.SetCollisionMesh` _bp_collisioncomponent (`self.GetItemMesh`))
  (`/Game/CombatSystem/Blueprints/Components/BP_CollisionComponent.AddActorToIgnore` _bp_collisioncomponent (`self.GetOwner`)))

(fn `UserConstructionScript`
  (`parent.UserConstructionScript`))