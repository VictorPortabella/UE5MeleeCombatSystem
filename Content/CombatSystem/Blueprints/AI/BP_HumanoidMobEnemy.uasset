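; Humanoid mob enemy Blueprint that extends a parent enemy with a melee weapon and a health bar shown only while targeted.
; The weapon collision component tracks the weapon mesh and deals stat-based point damage to hit actors that can receive it.
; Toggling combat snaps the weapon between hand and attach sockets.
; On death, the weapon switches to physics simulation.
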(event `self.ReceiveBeginPlay`
  (`parent.ReceiveBeginPlay`)
  (`/Game/CombatSystem/Blueprints/Components/BP_CollisionComponent.SetCollisionMesh` (`self.MainWeaponCollisionComponent`) (`self.WeaponMesh`))
  (bind _returnvalue (`|CreateWidget` "/Game/CombatSystem/UI/WP_HealthBar.WP_HealthBar_C" (`GameplayStatics.GetPlayerController` 0) false (`self.StatsComponent`)))
  (`WidgetComponent.SetWidget` (`self.HealthBar`) _returnvalue))

(event `/Game/CombatSystem/Blueprints/Interfaces/Targeting_BPI.OnTargeted`
  (params (bIsTargeted :type Boolean))
  (`parent.OnTargeted` bIsTargeted)
  (`SceneComponent.SetVisibility` (`self.HealthBar`) bIsTargeted false))

(event `self.MainWeaponCollisionComponent.OnHit`
  (params (HitResult :type "HitResult Structure"))
  (bind (_bblockinghit _binitialoverlap _time _distance _location _impactpoint _normal _impactnormal _physmat _hitactor) (`GameplayStatics.BreakHitResult` HitResult))
  (bind _canreceivedamage (message `/Game/CombatSystem/Blueprints/Interfaces/Combat_BPI.CanReceiveDamage` _hitactor))
  (if _canreceivedamage
    (`GameplayStatics.ApplyPointDamage` _hitactor (`/Game/CombatSystem/Blueprints/Components/BP_StatsComponent.GetCurrentStatValue` (`self.StatsComponent`) "NewEnumerator4") (`self.GetActorForwardVector` (`self.GetOwner`)) HitResult (`self.GetInstigatorController`) self (`self.Damage Type Class`))))

(event `SimulateWeaponPhysics`
  (bind _weaponmesh (`self.WeaponMesh`))
  (`PrimitiveComponent.SetCollisionProfileName` _weaponmesh "PhysicsActor" true)
  (`PrimitiveComponent.SetSimulatePhysics` _weaponmesh true))

(event `self.PerformDeath`
  (`parent.PerformDeath`)
  (`self.SimulateWeaponPhysics`))

(event `/Game/CombatSystem/Blueprints/Interfaces/Combat_BPI.ToggleCombat`
  (`parent.ToggleCombat`)
  (`SceneComponent.K2_AttachToComponent` (`self.WeaponMesh`) (`self.Mesh`) (select `bool` (`/Game/CombatSystem/Blueprints/Components/BP_CombatComponent.GetIsCombatEnabled` (`self.CombatComponent`)) :`false` (`self.AttachSocketName`) :`true` (`self.HandSocketName`)) "SnapToTarget" "SnapToTarget" "SnapToTarget" true))

(fn `UserConstructionScript`
  (`parent.UserConstructionScript`))