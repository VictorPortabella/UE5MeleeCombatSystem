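; BP_BossEnemy is a boss enemy that extends its parent AI character with a melee weapon and an on-screen health bar.
; A health widget bound to StatsComponent shows only while the boss is alive and has a valid target.
; MainWeaponCollisionComponent hits apply stat-based point damage to receptive actors, and combat toggles swap the weapon between hand and attach sockets.
; On death, the weapon simulates physics and the health bar hides.
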(event `self.ReceiveBeginPlay`
  (`parent.ReceiveBeginPlay`)
  (`/Game/CombatSystem/Blueprints/Components/BP_CollisionComponent.SetCollisionMesh` (`self.MainWeaponCollisionComponent`) (`self.WeaponMesh`))
  (bind _returnvalue (`|GenericCreateObject` (`GameplayStatics.GetPlayerController` 0) "/Game/CombatSystem/UI/WB_BossHealth.WB_BossHealth_C"))
  (set `self.BothHealthUI` _returnvalue)
  (`UserWidget.AddToViewport` _returnvalue 0)
  (`/Game/CombatSystem/UI/WB_BossHealth.Initialize` _returnvalue (`self.StatsComponent`)))

(event `SetBossHealthVisibility`
  (params (IsVisible :type Boolean))
  (bind _bothhealthui (`self.BothHealthUI`)
    (:`then`
      (`Widget.SetVisibility` _bothhealthui (select `bool` (and IsVisible (not (`/Game/CombatSystem/Blueprints/Components/BP_StateManagerComponent.GetIsDead` (`self.StateManagerComponent`)))) :`false` "Hidden" :`true` "SelfHitTestInvisible" :!type "ESlateVisibility Enum")))
    (:`else`)))

(event `self.MainWeaponCollisionComponent.OnHit`
  (params (HitResult :type "HitResult Structure"))
  (bind (_bblockinghit _binitialoverlap _time _distance _location _impactpoint _normal _impactnormal _physmat _hitactor) (`GameplayStatics.BreakHitResult` HitResult))
  (bind _canreceivedamage (message `/Game/CombatSystem/Blueprints/Interfaces/Combat_BPI.CanReceiveDamage` _hitactor))
  (if _canreceivedamage
    (`GameplayStatics.ApplyPointDamage` _hitactor (`/Game/CombatSystem/Blueprints/Components/BP_StatsComponent.GetCurrentStatValue` (`self.StatsComponent`) "NewEnumerator4") (`self.GetActorForwardVector` (`self.GetOwner`)) HitResult (`self.GetInstigatorController`) self (`self.Damage Type Class`))))

(event `SimulateWeaponPhysics`
  (bind _weaponmesh (`self.WeaponMesh`))
  (`PrimitiveComponent.SetCollisionProfileName` _weaponmesh "PhysicsActor" true)
  (`PrimitiveComponent.SetSimulatePhysics` _weaponmesh true))

(event `self.PerformDeath`
  (`parent.PerformDeath`)
  (`self.SimulateWeaponPhysics`)
  (`self.SetBossHealthVisibility` false))

(event `self.CombatComponent.OnCombatToggle`
  (params (bIsCombatEnabled :type Boolean))
  (`SceneComponent.K2_AttachToComponent` (`self.WeaponMesh`) (`self.Mesh`) (select `bool` bIsCombatEnabled :`false` (`self.AttachSocketName`) :`true` (`self.HandSocketName`)) "SnapToTarget" "SnapToTarget" "SnapToTarget" true))

(event `self.OnTargetSet`
  (params (NewTarget :type "Actor Object Reference"))
  (`parent.OnTargetSet` NewTarget)
  (`self.SetBossHealthVisibility` (`KismetSystemLibrary.IsValid` NewTarget)))

(fn `UserConstructionScript`
  (`parent.UserConstructionScript`))