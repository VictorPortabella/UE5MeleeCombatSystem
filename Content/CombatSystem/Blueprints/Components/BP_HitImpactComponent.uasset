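; Character component that handles hit reactions, combining sound, particles, montages and partial physical animation on the struck bone.
; ReceiveHit finds the nearest physics-asset bone and reduces a posture stat, whose result selects impact or stun montages, with optional timed posture recovery.
; Non-immune bones get damage-scaled impulses, while Tick drives a curve-based physics blend that accumulates over hits until timeout.
; PlayDeath stops reactions and applies the ragdoll profile.
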(event `self.ReceiveBeginPlay`
  ;[1 1 1] Begin Play
  (bind _ascharacter (cast `Character` (`self.GetOwner`)))
  (bind _returnvalue (`|AddComponentByClass` _ascharacter "/Script/Engine.PhysicalAnimationComponent"))
  (set `self.PhysicalAnimationComponent` _returnvalue)
  (set `self.OwnerMeshComponent` (`Character.Mesh` _ascharacter))
  (`PhysicalAnimationComponent.SetSkeletalMeshComponent` (`self.PhysicalAnimationComponent`) (`self.OwnerMeshComponent`))
  (set `self.StatsComponent` (`Actor.GetComponentByClass` _ascharacter "/Game/CombatSystem/Blueprints/Components/BP_StatsComponent.BP_StatsComponent_C")))

(event `self.ReceiveTick`
  (params (DeltaSeconds :type "Float (single-precision)"))
  ;[1 1 1] Tick: Lerp Blend Weight
  (if (not (`self.bIsDeath`))
    (set `self.HitReactionTimeRemaining` (- (`self.HitReactionTimeRemaining`) DeltaSeconds))
    (if (<= (`self.HitReactionTimeRemaining`) 0.0)
      (`self.DisableHitImpactPhysics`)
      (else
        (`SkeletalMeshComponent.SetAllBodiesBelowPhysicsBlendWeight` (`self.OwnerMeshComponent`) (`self.PelvisBone`) (* (`CurveFloat.GetFloatValue` (`self.CurvePhysicalBlendWeight`) (`KismetMathLibrary.FClamp` (- 1.0 (/ (`self.HitReactionTimeRemaining`) (`self.HitReactionDuration`))))) (`self.CurrentMaxBlendWeight`)) false true)))))

(event `ReceiveHit`
  (params (HitInfo :type "HitResult Structure") (Damage :type "Float (double-precision)"))
  ;[1 1 1] ReceiveHit
  (set `self.LastHitInfo` HitInfo)
  (set `self.LastDamage` Damage)
  (`self.SetHitImpactBone`)
  (`self.ApplyImpactEffect`)
  (if (not (`self.bIsDeath`))
    (bind _bisempty (`/Game/CombatSystem/Blueprints/Components/BP_StatsComponent.ModifyCurrentStatValue` (`self.StatsComponent`) "NewEnumerator2" (* (`self.LastDamage`) -1.0) true))
    (if _bisempty
      (`self.SimulateHitImpactPhysics` 1.0)
      (`self.PlayHitStunMontage`)
      (if (`self.bResetStatOnEmpty`)
        (bind _returnvalue (`KismetSystemLibrary.K2_SetTimerDelegate` (delegate `RecoverPostureEvent`) (`self.TimeToRecoverPosture`)))
        (set `self.TimerHandle_RecoverPosture` _returnvalue))
      (else
        (`self.SimulateHitImpactPhysics` 1.0)
        (`self.PlayHitImpactMontage`)))))

(event `RecoverPostureEvent`
  ;[1 1 1] ReceiveHit
  (`/Game/CombatSystem/Blueprints/Components/BP_StatsComponent.ResetStat` (`self.StatsComponent`) "NewEnumerator2"))

(event `PlayHitImpactMontage`
  ;[1 1 1] PlayAnim
  (message `/Game/CombatSystem/Blueprints/Interfaces/HitImpact_BPI.PerformHitImpact` (`self.GetOwner`) (`self.Get Anim by Bone` (`self.LastHitImpactBone`) (`self.HitImpactAnims`) (`self.DefaultHitImpact`)) false))

(event `PlayHitStunMontage`
  ;[1 1 1] PlayAnim
  (bind (_duration _bsuccess) (message `/Game/CombatSystem/Blueprints/Interfaces/HitImpact_BPI.PerformHitImpact` (`self.GetOwner`) (`self.Get Anim by Bone` (`self.LastHitImpactBone`) (`self.HitStunAnims`) (`self.DefaultHitStun`)) true))
  (if _bsuccess
    (`self.OnPlayingHitStun` true)
    (bind _returnvalue (`KismetSystemLibrary.K2_SetTimerDelegate` (delegate `OnFinishHitStun`) _duration))
    (set `self.Handle_FinishHitStune` _returnvalue)))

(event `OnFinishHitStun`
  ;[1 1 1] PlayAnim
  (`self.OnPlayingHitStun` false))

(event `ApplyImpactEffect`
  ;[1 1 1] Visual And Audio
  (`GameplayStatics.PlaySoundAtLocation` (`self.HitImpactAudio`) (`.ImpactPoint` (`GameplayStatics.BreakHitResult` (`self.LastHitInfo`))) (struct) 1.0 1.0 0.0 null null null null)
  (`NiagaraFunctionLibrary.SpawnSystemAttached` (`KismetArrayLibrary.Array_Random` (`self.HitImpactParticles`)) (`self.OwnerMeshComponent`) (`self.LastHitImpactBone`) (0.0 0.0 0.0) (struct) "KeepRelativeOffset"))

(fn `CanApplyPhysicalAnimations`
  (returns (bCanApply :type Boolean))
  (bind _lasthitimpactbone (`self.LastHitImpactBone`))
  (for _array_element (`self.InmuneParentBones`)
    (if (or (== _array_element _lasthitimpactbone) (`SkinnedMeshComponent.BoneIsChildOf` (`self.OwnerMeshComponent`) _lasthitimpactbone _array_element))
      (return false)))
  (return true))

(fn `DisableHitImpactPhysics`
  (set `self.HitReactionTimeRemaining` 0.0)
  (set `self.CurrentMaxBlendWeight` 0.0)
  (`SkeletalMeshComponent.SetAllBodiesSimulatePhysics` (`self.OwnerMeshComponent`) false)
  (`self.SetComponentTickEnabled` false))

(fn `Get Anim by Bone`
  (params (BoneName :type Name) (InHitImpactAnims :type "Array of /Game/CombatSystem/Blueprints/Structs/F_AnimByBones Structure") (InDefaultAnim :type "AnimMontage Object Reference"))
  (returns (AnimMontage :type "AnimMontage Object Reference"))
  (for _array_element InHitImpactAnims
    (bind (_animmontage _bones) (break `/Game/CombatSystem/Blueprints/Structs/F_AnimByBones` _array_element))
    (for _array_element_2 _bones
      (if (== _array_element_2 (`local.BoneName`))
        (return _animmontage))))
  (return (`local.InDefaultAnim`)))

(fn `Get Last Hit Direction`
  (returns (Direction :type "Vector Structure"))
  (bind (_bblockinghit _binitialoverlap _time _distance _location _impactpoint _normal _impactnormal) (`GameplayStatics.BreakHitResult` (`self.LastHitInfo`)))
  (return (`KismetMathLibrary.GetDirectionUnitVector` (+ _impactpoint _impactnormal) _impactpoint)))

(fn `PlayDeath`
  (set `self.bIsDeath` true)
  (`self.DisableHitImpactPhysics`)
  (`PhysicalAnimationComponent.ApplyPhysicalAnimationProfileBelow` (`self.PhysicalAnimationComponent`) "None" (`self.RagdollProfileName`) true false))

(fn `SetHitImpactBone`
  ;[1 1 1] Get Hit Bone
  (bind _ascharacter (cast `Character` (`self.GetOwner`)))
  (bind (_closestworldposition _normal _bonename) (`SkeletalMeshComponent.K2_GetClosestPointOnPhysicsAsset` (`Character.Mesh` _ascharacter) (`.ImpactPoint` (`GameplayStatics.BreakHitResult` (`self.LastHitInfo`)))))
  (set `self.LastHitImpactBone` (select `bool` (and (!= _bonename (`self.RootBone`)) (!= _bonename (`self.PelvisBone`))) :`false` (`self.SpineBone`) :`true` _bonename)))

(fn `SimulateHitImpactPhysics`
  (params (MaxRatio :type "Float (double-precision)" :default 1.0))
  (locals (HitDir :type "Vector Structure") (Impulse :type "Vector Structure"))
  (if (`self.CanApplyPhysicalAnimations`)
    ;[1 1 1] Enable Physics
    (set `self.CurrentMaxBlendWeight` (`KismetMathLibrary.FClamp` (+ (`self.CurrentMaxBlendWeight`) (`self.IncreaseBlendWeightByHit`)) 0.0 (`local.MaxRatio`)))
    (set `self.HitReactionTimeRemaining` (`self.HitReactionDuration`))
    (`PrimitiveComponent.SetCollisionProfileName` (`self.OwnerMeshComponent`) "Ragdoll" true)
    (`PhysicalAnimationComponent.ApplyPhysicalAnimationProfileBelow` (`self.PhysicalAnimationComponent`) (`self.PelvisBone`) (`self.Hit Reaction Profile Name`) false false)
    (`SkeletalMeshComponent.SetAllBodiesBelowSimulatePhysics` (`self.OwnerMeshComponent`) (`self.LastHitImpactBone`) true true)
    ;[1 1 1] Apply Impulse
    (set `local.HitDir` (`self.Get Last Hit Direction`))
    (set `local.Impulse` (* (`local.HitDir`) (* (`self.HitStrengthByDamage`) (`self.LastDamage`))))
    (`PrimitiveComponent.AddImpulse` (`self.OwnerMeshComponent`) (`local.Impulse`) (`self.LastHitImpactBone`) false)
    (`self.SetComponentTickEnabled` true)))